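; Lobby workshop shop Blueprint for recipes that highlights itself with a spotlight while being interacted with.
; It extends a parent interactable, calling the parent on construction and on interaction begin and end.
; Interaction begin sets the spotlight to double the configured interact light intensity, and interaction end turns it off.
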(fn `InteractBegin`
  (`parent.InteractBegin`)
  (`LightComponent.SetIntensity` (`self.SpotLight`) (* (`self.InteractLightIntensity`) 2.0)))

(fn `InteractEnd`
  (`parent.InteractEnd`)
  (`LightComponent.SetIntensity` (`self.SpotLight`) 0.0))

(fn `UserConstructionScript`
  (`parent.UserConstructionScript`))