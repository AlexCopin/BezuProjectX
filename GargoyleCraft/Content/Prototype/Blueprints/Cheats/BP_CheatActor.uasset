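; BP_CheatActor is a prototype actor that hosts the on-screen cheat menu.
; On BeginPlay it creates WBP_Cheat_Main for the first player controller, adds it to the viewport and starts it collapsed.
; The C key drives a FlipFlop that switches the widget between visible (not hit-testable itself) and collapsed.
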(event `self.ReceiveBeginPlay`
  (bind _returnvalue (`|CreateWidget` "/Game/Prototype/Blueprints/Cheats/UI/WBP_Cheat_Main.WBP_Cheat_Main_C" (`GameplayStatics.GetPlayerController` 0)))
  (bind _output_get (set `self.CheatWidgets` _returnvalue))
  (`UserWidget.AddToViewport` _output_get 10)
  (`Widget.SetVisibility` _output_get "Collapsed"))

(event `Key|C`
  (params (Key :type "Key Structure"))
  (:`Pressed`
    (`/Engine/EditorBlueprintResources/StandardMacros.FlipFlop`
      (:`A`
        (`Widget.SetVisibility` (`self.CheatWidgets`) "SelfHitTestInvisible"))
      (:`B`
        (`Widget.SetVisibility` (`self.CheatWidgets`) "Collapsed")))))

(fn `UserConstructionScript`)