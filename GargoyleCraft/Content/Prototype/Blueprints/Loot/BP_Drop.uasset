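; BP_Drop is a prototype loot drop actor that bobs continuously in place.
; BeginPlay caches the spawn location and a float target with the same X and Y but a fixed world Z, not a relative offset.
; Tick accumulates running time and moves the actor between the two points without sweep, using a sine remapped to 0–1 as the lerp alpha.
; It has no pickup or overlap logic.
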(event `self.ReceiveBeginPlay`
  (bind _output_get (set `self.InitialLocation` (`self.K2_GetActorLocation`)))
  (set `self.FloatingLocation` (`KismetMathLibrary.MakeVector` (.x _output_get) (.y _output_get) 150.0)))

(event `self.ReceiveTick`
  (params (DeltaSeconds :type "Float (single-precision)"))
  (bind _output_get (set `self.RunningTime` (+ DeltaSeconds (`self.RunningTime`))))
  (`self.K2_SetActorLocation` (`KismetMathLibrary.VLerp` (`self.InitialLocation`) (`self.FloatingLocation`) (+ (* (`KismetMathLibrary.Sin` _output_get) 0.5) 0.5))))

(fn `UserConstructionScript`)