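; BP_Interactible is a prototype interactible actor that lights up while the top-down player character overlaps it.
; The construction script registers its base point light in an array, which the interaction functions loop over.
; Overlap begin and end, filtered by a cast to BP_TopDownCharacter, call InteractBegin and InteractEnd.
; These set every light to the interact intensity or to zero, and print a debug message with the object name.
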(event `self.ReceiveActorBeginOverlap`
  (params (OtherActor :type "Actor Object Reference"))
  (cast `/Game/Prototype/Blueprints/BP_TopDownCharacter` OtherActor)
  (`self.InteractBegin`))

(event `self.ReceiveActorEndOverlap`
  (params (OtherActor :type "Actor Object Reference"))
  (cast `/Game/Prototype/Blueprints/BP_TopDownCharacter` OtherActor)
  (`self.InteractEnd`))

(fn `InteractBegin`
  (`KismetSystemLibrary.PrintString` (`KismetStringLibrary.Concat_StrStr` "BeginInteract - " (`KismetSystemLibrary.GetObjectName` self)))
  (for _array_element (`self.PointLightsArray`)
    (`LightComponent.SetIntensity` _array_element (`self.InteractLightIntensity`))))

(fn `InteractEnd`
  (`KismetSystemLibrary.PrintString` (`KismetStringLibrary.Concat_StrStr` "EndInteract - " (`KismetSystemLibrary.GetObjectName` self)))
  (for _array_element (`self.PointLightsArray`)
    (`LightComponent.SetIntensity` _array_element 0.0)))

(fn `UserConstructionScript`
  (`KismetArrayLibrary.Array_AddUnique` (`self.PointLightsArray`) (`self.PointLightBase`)))