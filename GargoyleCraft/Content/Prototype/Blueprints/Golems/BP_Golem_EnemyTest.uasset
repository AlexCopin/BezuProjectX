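; BP_Golem_EnemyTest is a prototype test enemy golem that initializes from the DA_GolemTest data asset, using its spawn location as the first target location.
; On BeginPlay it caches its original mesh material, binds its attribute bar widget to itself and subscribes to the RTS player controller's golem added and removed events.
; Those events swap one material slot to the selected material or back when the golem concerned is itself.
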(event `self.ReceiveBeginPlay`
  (`|ExecutionSequence`
    (:`then_0`
      (set `self.OriginalMat` (`|GetArrayItem` (`MeshComponent.GetMaterials` (`self.Mesh`)) (`self.IndexMaterialToChange`)))
      (bind _aswbp_attribute_bar_golem (cast `/Game/Prototype/Blueprints/Golems/UI/WBP_AttributeBar_Golem` (`WidgetComponent.GetWidget` (`self.AttributeBar`))))
      (`/Game/Prototype/Blueprints/Golems/UI/WBP_AttributeBar_Golem.Init` _aswbp_attribute_bar_golem self)
      (bind _asgc_pc_rts (cast `GC_PC_RTS` (`GameplayStatics.GetPlayerController` 0)))
      (add `GC_PC_RTS.OnGolemAdded` _asgc_pc_rts (delegate `OnGolemAdded_Event`))
      (add `GC_PC_RTS.OnGolemRemoved` _asgc_pc_rts (delegate `OnGolemRemoved_Event`)))
    (:`then_1`
      (`self.Init` "/Game/Prototype/Blueprints/Golems/GolemList/DA_GolemTest.DA_GolemTest" (`self.K2_GetActorLocation`)))))

(event `OnGolemAdded_Event`
  (params (Golem :type "Golem Object Reference"))
  (if (== Golem self)
    (`PrimitiveComponent.SetMaterial` (`self.Mesh`) (`self.IndexMaterialToChange`) (`self.SelectedMat`))))

(event `OnGolemRemoved_Event`
  (params (Golem :type "Golem Object Reference"))
  (if (== Golem self)
    (`PrimitiveComponent.SetMaterial` (`self.Mesh`) (`self.IndexMaterialToChange`) (`self.OriginalMat`))))

(fn `UserConstructionScript`)