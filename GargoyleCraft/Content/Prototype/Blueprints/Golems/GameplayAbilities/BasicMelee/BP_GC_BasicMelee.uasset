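; Gameplay cue for the golem basic melee ability, showing an effect and debug boxes at the cue location.
; OnActive moves the Effect component to that location, activates it and briefly draws a small debug box rotated to match the instigator.
; OnExecute only draws a larger, longer-lasting debug box at the location.
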(fn `OnActive`
  (params (MyTarget :type "Actor Object Reference") (Parameters :type "GameplayCueParameters Structure (by ref)"))
  (returns (ReturnValue :type Boolean))
  (bind (_normalizedmagnitude _rawmagnitude _effectcontext _matchedtagname _originaltag _aggregatedsourcetags _aggregatedtargettags _location _normal _instigator) (`AbilitySystemBlueprintLibrary.BreakGameplayCueParameters` Parameters))
  (bind _effect (`self.Effect`))
  (`SceneComponent.K2_SetWorldLocation` _effect _location false false)
  (`ActorComponent.Activate` _effect true)
  (`KismetSystemLibrary.DrawDebugBox` null _location (20.0 20.0 20.0) (struct :`R` 1.0 :`B` 0.12442 :`A` 1.0) (`self.K2_GetActorRotation` _instigator) 0.5 1.0)
  (return true))

(fn `OnExecute`
  (params (MyTarget :type "Actor Object Reference") (Parameters :type "GameplayCueParameters Structure (by ref)"))
  (returns (ReturnValue :type Boolean))
  (`KismetSystemLibrary.DrawDebugBox` null (`.Location` (`AbilitySystemBlueprintLibrary.BreakGameplayCueParameters` Parameters)) (100.0 100.0 100.0) (struct :`R` 1.0 :`B` 0.12442 :`A` 1.0) (struct) 2.0 10.0)
  (return true))

(fn `UserConstructionScript`)