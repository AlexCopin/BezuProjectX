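; BP_Golem is a prototype golem unit that can be selected and deselected by an RTS player controller.
; Selected adds the golem to GC_PC_RTS's selected-golem list, swaps the mesh's first material slot to SelectedMat and returns itself.
; Deselect removes it from that list and restores the original material cached at BeginPlay.
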(event `self.ReceiveBeginPlay`
  (set `self.OriginalMat` (`|GetArrayItem` (`MeshComponent.GetMaterials` (`self.Mesh`)))))

(event `self.ReceiveTick`
  (params (DeltaSeconds :type "Float (single-precision)")))

(event `/Game/Prototype/Blueprints/Interfaces/BPI_Selected.Deselect`
  (params (PlayerController :type "PlayerController Object Reference"))
  (bind _asgc_pc_rts (cast `GC_PC_RTS` PlayerController))
  (`GC_PC_RTS.RemoveFromSelectedGolems` _asgc_pc_rts self)
  (`PrimitiveComponent.SetMaterial` (`self.Mesh`) 0 (`self.OriginalMat`)))

(fn `Selected`
  (params (PlayerController :type "PlayerController Object Reference"))
  (returns (ActorSelected :type "Actor Object Reference"))
  (bind _asgc_pc_rts (cast `GC_PC_RTS` PlayerController))
  (`GC_PC_RTS.AddToSelectedGolems` _asgc_pc_rts self)
  (`PrimitiveComponent.SetMaterial` (`self.Mesh`) 0 (`self.SelectedMat`))
  (return self))

(fn `UserConstructionScript`)