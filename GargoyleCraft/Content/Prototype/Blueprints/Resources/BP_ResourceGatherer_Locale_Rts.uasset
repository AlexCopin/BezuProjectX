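; BP_ResourceGatherer_Locale_Rts is a resource gatherer that adds UI feedback on top of its parent's gathering logic.
; Initialize links its WBP_ResourceGatherer widget component to itself and caches the resource icon from GCPlayerDataSubsystem via the resource tag.
; Each Gather spawns a WBP_ResourceAdded popup at the mouse position, showing that icon and the gathered quantity.
; Terminate destroys the widget component.
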(event `self.Initialize`
  (params (DataSent :type "PlayerData Structure"))
  (bind (_returnvalue_quantity _returnvalue_pda_resource) (break `ResourceData` (`GC_PlayerDataSubsystem.GetResourceData` (subsystem `GC_PlayerDataSubsystem`) (`self.ResourceTag`))))
  (bind (_returnvalue_title _returnvalue_description _returnvalue_flavor _returnvalue_icon) (break `TooltipData` (`PDA_Generic.GetTooltip` _returnvalue_pda_resource)))
  (`parent.Initialize` DataSent)
  (bind _aswbp_resource_gatherer (cast `/Game/Prototype/Blueprints/Resources/Widgets/WBP_ResourceGatherer` (`WidgetComponent.GetWidget` (`self.Widget`))))
  (`/Game/Prototype/Blueprints/Resources/Widgets/WBP_ResourceGatherer.SetGatherer` _aswbp_resource_gatherer self)
  (set `self.ResourceIconTexture` _returnvalue_icon))

(event `self.Terminate`
  (`parent.Terminate`)
  (`ActorComponent.K2_DestroyComponent` (`self.Widget`)))

(event `self.Gather`
  (`parent.Gather`)
  (bind _returnvalue (`|CreateWidget` "/Game/Prototype/Blueprints/Resources/Widgets/WBP_ResourceAdded.WBP_ResourceAdded_C" null (`self.ResourceIconTexture`) (`self.QuantityResource`)))
  (`UserWidget.AddToViewport` _returnvalue 2)
  (bind _returnvalue_2 (`WidgetLayoutLibrary.GetMousePositionOnViewport`))
  (`UserWidget.SetPositionInViewport` _returnvalue _returnvalue_2 true))

(fn `UserConstructionScript`)