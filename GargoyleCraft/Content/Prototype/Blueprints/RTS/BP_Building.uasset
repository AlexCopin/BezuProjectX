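; BP_Building is a prototype RTS building that spawns golems and offers a troop-choice widget.
; Initialize fills that widget from the army's golem types, falling back to a test asset, then saves player data.
; Selection toggles the widget and spawn flag and binds right-click to move the golem spawn point to the terrain cursor, with a debug line drawn to it.
; The data-initialized subscription never runs.
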(event `self.ReceiveBeginPlay`)

(event `SpawnGolem`
  (params (GolemClass :type "PDA_Golem Soft Object Reference"))
  (`self.RequestGolemCreation` GolemClass))

(event `self.ReceiveTick`
  (params (DeltaSeconds :type "Float (single-precision)"))
  (if (`self.bIsSelected`)
    (`KismetSystemLibrary.DrawDebugLine` (`SceneComponent.K2_GetComponentLocation` (`self.RootComponent`)) (`SceneComponent.K2_GetComponentLocation` (`self.GolemSpawnFlag`)) (struct :`A` 1.0))))

(event `OnPCRightClick`
  (`SceneComponent.K2_SetWorldLocation` (`self.GolemSpawnFlag`) (`/Game/Prototype/Blueprints/RTS/BP_PC_RTS.CursorOnTerrainLocation` (`self.OwnerPC`)) false false))

(event `DataInitialized`
  (params (DataSent :type "PlayerData Structure")))

(event `self.Initialize`
  (params (DataSent :type "PlayerData Structure"))
  (bind (_armydata_name _armydata_description _armydata_nbavailableslots _armydata_tagsunlocked _armydata_golemtypesinarmy) (break `ArmyData` (break `PlayerData` DataSent)))
  (if (`KismetArrayLibrary.Array_IsEmpty` _armydata_golemtypesinarmy)
    (set `self.GolemPool` (`|MakeArray` "/Game/Prototype/Blueprints/Golems/GolemList/DA_GolemTest.DA_GolemTest" :!type "PDA_Golem Object Reference"))
    (else
      (set `self.GolemPool` _armydata_golemtypesinarmy)))
  (bind _aswbp_building_troop_choice (cast `/Game/Prototype/Blueprints/RTS/Widgets/WBP_Building_TroopChoice` (`WidgetComponent.GetWidget` (`self.Widget`))))
  (`PanelWidget.ClearChildren` (`/Game/Prototype/Blueprints/RTS/Widgets/WBP_Building_TroopChoice.ButtonContainer` _aswbp_building_troop_choice))
  (`/Game/Prototype/Blueprints/RTS/Widgets/WBP_Building_TroopChoice.Init` :`self` _aswbp_building_troop_choice :`Pool` (`self.GolemPool`) :`Building` self)
  (`SceneComponent.SetVisibility` (`self.SpawnFlag`) false false)
  (`SceneComponent.SetVisibility` (`self.Widget`) false false)
  (`GC_SaveSubsystem.SavePlayerData` (subsystem `GC_SaveSubsystem`)))

(fn `Selected`
  (params (PlayerController :type "GC_PC_RTS Object Reference"))
  (returns (ReturnValue :type "Actor Object Reference"))
  (bind _asbp_pc_rts (cast `/Game/Prototype/Blueprints/RTS/BP_PC_RTS` PlayerController))
  (bind _output_get (set `self.OwnerPC` _asbp_pc_rts))
  (add `/Game/Prototype/Blueprints/RTS/BP_PC_RTS.Event_RightClickPC` _output_get (`|CreateDelegate` :!event `OnPCRightClick`))
  (`SceneComponent.SetVisibility` (`self.SpawnFlag`) true false)
  (set `self.bIsSelected` true)
  (`SceneComponent.SetVisibility` (`self.Widget`) true false)
  (return self))

(fn `Unselected`
  (params (PlayerController :type "GC_PC_RTS Object Reference"))
  (returns (ReturnValue :type "Actor Object Reference"))
  (bind _asbp_pc_rts (cast `/Game/Prototype/Blueprints/RTS/BP_PC_RTS` PlayerController))
  (bind _output_get (set `self.OwnerPC` _asbp_pc_rts))
  (remove `/Game/Prototype/Blueprints/RTS/BP_PC_RTS.Event_RightClickPC` _output_get (`|CreateDelegate` :!event `OnPCRightClick`))
  (`SceneComponent.SetVisibility` (`self.SpawnFlag`) false false)
  (set `self.bIsSelected` false)
  (`SceneComponent.SetVisibility` (`self.Widget`) false false)
  (return self))

(fn `UserConstructionScript`)