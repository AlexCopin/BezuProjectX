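; RTS player controller that shows the mouse cursor and handles click selection, adding camera and building input mappings on start.
; Each tick it traces under the cursor on the Camera channel, caching the hit actor and terrain location, marked with a debug sphere.
; Select input deselects the current actor and selects the hovered one through BPI_Selected.
; MoveFlag input fires the RightClickPC event dispatcher.
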(event `self.ReceiveBeginPlay`
  (bind _returnvalue (pcsubsystem `EnhancedInputLocalPlayerSubsystem` self))
  (`EnhancedInputSubsystemInterface.AddMappingContext` _returnvalue "/Game/Prototype/Input/IMC_RTS_Camera.IMC_RTS_Camera" 0 (struct))
  (`EnhancedInputSubsystemInterface.AddMappingContext` _returnvalue "/Game/Prototype/Input/IMC_RTS_Buildings.IMC_RTS_Buildings" 0 (struct))
  (set `self.bShowMouseCursor` true)
  (bind _asbp_pawn_rts (cast `/Game/Prototype/Blueprints/RTS/BP_Pawn_RTS` (`self.K2_GetPawn`)))
  (bind _output_get (set `self.PlayerPawn` _asbp_pawn_rts))
  (set `self.PawnCamera` (`/Game/Prototype/Blueprints/RTS/BP_Pawn_RTS.Camera` _output_get)))

(event `self.ReceiveTick`
  (params (DeltaSeconds :type "Float (single-precision)"))
  (bind (_bblockinghit _binitialoverlap _time _distance _location _impactpoint _normal _impactnormal _physmat _hitactor) (`GameplayStatics.BreakHitResult` (`self.GetHitResultUnderCursorByChannel` "TraceTypeQuery2")))
  (bind _output_get (set `self.CursorOnTerrainLocation` _location))
  (`KismetSystemLibrary.DrawDebugSphere` _output_get 20.0 12 (struct :`R` 1.0 :`A` 1.0))
  (bind _output_get_2 (set `self.CurrentHitActor` _hitactor)))

(event `EnhancedInput|/Game/Prototype/Input/Actions/IA_RTS_Select`
  (params (ActionValue :type Boolean) (ElapsedSeconds :type "Float (double-precision)") (TriggeredSeconds :type "Float (double-precision)") (InputAction :type "InputAction Object Reference" :default "/Game/Prototype/Input/Actions/IA_RTS_Select.IA_RTS_Select"))
  (bind _actorselected (`self.ActorSelected`))
  (bind _currenthitactor (`self.CurrentHitActor`))
  (:`Completed`
    (`/Engine/EditorBlueprintResources/StandardMacros.IsValid` _actorselected
      (:`Is Valid`
        (bind _asbpi_selected (cast `/Game/Prototype/Blueprints/Interfaces/BPI_Selected` _actorselected))
        (`/Game/Prototype/Blueprints/Interfaces/BPI_Selected.Deselect` _asbpi_selected self))
      (:`Is Not Valid`
        _))
    (`/Engine/EditorBlueprintResources/StandardMacros.IsValid` _currenthitactor
      (:`Is Valid`
        (bind _asbpi_selected_2 (cast `/Game/Prototype/Blueprints/Interfaces/BPI_Selected` _currenthitactor))
        (bind _actorselected_2 (`/Game/Prototype/Blueprints/Interfaces/BPI_Selected.Selected` _asbpi_selected_2 self))
        (set `self.ActorSelected` _actorselected_2)))))

(event `EnhancedInput|/Game/Prototype/Input/Actions/IA_RTS_MoveFlag`
  (params (ActionValue :type Boolean) (ElapsedSeconds :type "Float (double-precision)") (TriggeredSeconds :type "Float (double-precision)") (InputAction :type "InputAction Object Reference" :default "/Game/Prototype/Input/Actions/IA_RTS_MoveFlag.IA_RTS_MoveFlag"))
  (:`Completed`
    (`self.Event_RightClickPC`)))

(fn `UserConstructionScript`)