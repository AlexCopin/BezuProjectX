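; RTS camera pawn prototype that pans and yaws from Enhanced Input actions.
; Move actions set a target location along world X/Y, and rotate actions set a target yaw, each offset by a speed variable.
; Tick lerps location and rotation using normalized-vector lengths as alpha, normally 1 rather than time-based.
; Location therefore tends to snap to target, while the rotation lerp's reversed inputs favor the current rotation.
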(event `self.ReceiveBeginPlay`
  (set `self.ProcessingLocation` (`self.K2_GetActorLocation`)))

(event `self.ReceiveTick`
  (params (DeltaSeconds :type "Float (single-precision)"))
  (bind _returnvalue (`self.K2_GetActorLocation`))
  (bind _returnvalue_2 (`self.K2_GetActorRotation`))
  (bind _processinglocation (`self.ProcessingLocation`))
  (bind _processingrotation (`self.ProcessingRotation`))
  ;[1 1 1] Lerp movements
  (`self.K2_SetActorLocation` (`KismetMathLibrary.VLerp` _returnvalue _processinglocation (`KismetMathLibrary.VSize` (`KismetMathLibrary.Normal` (/ _returnvalue _processinglocation)))))
  (`self.K2_SetActorRotation` (`KismetMathLibrary.RLerp` _processingrotation _returnvalue_2 (`KismetMathLibrary.VSize` (`KismetMathLibrary.Normal` (/ (`KismetMathLibrary.GetRightVector` _processingrotation) (`KismetMathLibrary.GetRightVector` _returnvalue_2)))))))

(event `EnhancedInput|/Game/Prototype/Input/Actions/IA_CameraRotateLeft`
  (params (ActionValue :type Boolean) (ElapsedSeconds :type "Float (double-precision)") (TriggeredSeconds :type "Float (double-precision)") (InputAction :type "InputAction Object Reference" :default "/Game/Prototype/Input/Actions/IA_CameraRotateLeft.IA_CameraRotateLeft"))
  (bind (_returnvalue_roll _returnvalue_pitch _returnvalue_yaw) (`KismetMathLibrary.BreakRotator` (`self.K2_GetActorRotation`)))
  ;[1 1 1] Rotation
  (:`Triggered`
    (set `self.ProcessingRotation` (`KismetMathLibrary.MakeRotator` _returnvalue_roll _returnvalue_pitch (+ _returnvalue_yaw (`self.CameraRotateSpeed`))))))

(event `EnhancedInput|/Game/Prototype/Input/Actions/IA_CameraRotateRight`
  (params (ActionValue :type Boolean) (ElapsedSeconds :type "Float (double-precision)") (TriggeredSeconds :type "Float (double-precision)") (InputAction :type "InputAction Object Reference" :default "/Game/Prototype/Input/Actions/IA_CameraRotateRight.IA_CameraRotateRight"))
  (bind (_returnvalue_roll _returnvalue_pitch _returnvalue_yaw) (`KismetMathLibrary.BreakRotator` (`self.K2_GetActorRotation`)))
  ;[1 1 1] Rotation
  (:`Triggered`
    (set `self.ProcessingRotation` (`KismetMathLibrary.MakeRotator` _returnvalue_roll _returnvalue_pitch (- _returnvalue_yaw (`self.CameraRotateSpeed`))))))

(event `EnhancedInput|/Game/Prototype/Input/Actions/IA_CameraMoveDown`
  (params (ActionValue :type Boolean) (ElapsedSeconds :type "Float (double-precision)") (TriggeredSeconds :type "Float (double-precision)") (InputAction :type "InputAction Object Reference" :default "/Game/Prototype/Input/Actions/IA_CameraMoveDown.IA_CameraMoveDown"))
  (bind (_returnvalue_x _returnvalue_y _returnvalue_z) (`KismetMathLibrary.BreakVector` (`self.K2_GetActorLocation`)))
  ;[1 1 1] Move
  (:`Triggered`
    (set `self.ProcessingLocation` (`KismetMathLibrary.MakeVector` _returnvalue_x (+ _returnvalue_y (`self.CameraMoveSpeed`)) _returnvalue_z))))

(event `EnhancedInput|/Game/Prototype/Input/Actions/IA_CameraMoveUp`
  (params (ActionValue :type Boolean) (ElapsedSeconds :type "Float (double-precision)") (TriggeredSeconds :type "Float (double-precision)") (InputAction :type "InputAction Object Reference" :default "/Game/Prototype/Input/Actions/IA_CameraMoveUp.IA_CameraMoveUp"))
  (bind (_returnvalue_x _returnvalue_y _returnvalue_z) (`KismetMathLibrary.BreakVector` (`self.K2_GetActorLocation`)))
  ;[1 1 1] Move
  (:`Triggered`
    (set `self.ProcessingLocation` (`KismetMathLibrary.MakeVector` _returnvalue_x (- _returnvalue_y (`self.CameraMoveSpeed`)) _returnvalue_z))))

(event `EnhancedInput|/Game/Prototype/Input/Actions/IA_CameraMoveLeft`
  (params (ActionValue :type Boolean) (ElapsedSeconds :type "Float (double-precision)") (TriggeredSeconds :type "Float (double-precision)") (InputAction :type "InputAction Object Reference" :default "/Game/Prototype/Input/Actions/IA_CameraMoveLeft.IA_CameraMoveLeft"))
  (bind (_returnvalue_x _returnvalue_y _returnvalue_z) (`KismetMathLibrary.BreakVector` (`self.K2_GetActorLocation`)))
  ;[1 1 1] Move
  (:`Triggered`
    (set `self.ProcessingLocation` (`KismetMathLibrary.MakeVector` (- _returnvalue_x (`self.CameraMoveSpeed`)) _returnvalue_y _returnvalue_z))))

(event `EnhancedInput|/Game/Prototype/Input/Actions/IA_CameraMoveRight`
  (params (ActionValue :type Boolean) (ElapsedSeconds :type "Float (double-precision)") (TriggeredSeconds :type "Float (double-precision)") (InputAction :type "InputAction Object Reference" :default "/Game/Prototype/Input/Actions/IA_CameraMoveRight.IA_CameraMoveRight"))
  (bind (_returnvalue_x _returnvalue_y _returnvalue_z) (`KismetMathLibrary.BreakVector` (`self.K2_GetActorLocation`)))
  ;[1 1 1] Move
  (:`Triggered`
    (set `self.ProcessingLocation` (`KismetMathLibrary.MakeVector` (+ _returnvalue_x (`self.CameraMoveSpeed`)) _returnvalue_y _returnvalue_z))))

(fn `UserConstructionScript`)