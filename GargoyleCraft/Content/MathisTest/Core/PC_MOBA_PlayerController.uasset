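; MOBA player controller that pans the controlled pawn along world X and Y using movement axes or mouse edge-scrolling.
; The MOBA_MouseMovement axis event, used as a per-frame update, compares the cursor's viewport position to an edge threshold and sets forward and right scales.
; The MoveForward and MoveRight events feed AddMovementInput, using their axis value when non-zero and the mouse scale otherwise.
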(event `InputAxis|MOBA_MoveForward`
  (params (AxisValue :type "Float (single-precision)"))
  (`Pawn.AddMovementInput` (`self.K2_GetPawn`) (10.0 0.0 0.0) (`KismetMathLibrary.SelectFloat` AxisValue (`self.MouseForwardScale`) (!= AxisValue 0.0)) false))

(event `InputAxis|MOBA_MoveRight`
  (params (AxisValue :type "Float (single-precision)"))
  (`Pawn.AddMovementInput` (`self.K2_GetPawn`) (0.0 10.0 0.0) (`KismetMathLibrary.SelectFloat` AxisValue (`self.MouseRightScale`) (!= AxisValue 0.0)) false))

(event `InputAxis|MOBA_MouseMovement`
  (params (AxisValue :type "Float (single-precision)"))
  (bind (_returnvalue_x _returnvalue_y) (`KismetMathLibrary.BreakVector2D` (`WidgetLayoutLibrary.GetViewportSize`)))
  (bind (_locationx _locationy) (`self.GetMousePosition`))
  (bind _viewportedgethreshold (`self.ViewportEdgeThreshold`))
  (bind _viewportedgethreshold_2 (`self.ViewportEdgeThreshold`))
  (bind _returnvalue (/ _locationy _returnvalue_y))
  (bind _returnvalue_2 (/ _locationx _returnvalue_x))
  (if (< _returnvalue_2 _viewportedgethreshold_2)
    (set `self.MouseRightScale` -1.0)
    (elif (> _returnvalue_2 (- 1.0 _viewportedgethreshold_2))
      (set `self.MouseRightScale` 1.0)
      (else
        (set `self.MouseRightScale` 0.0))))
  (if (< _returnvalue _viewportedgethreshold)
    (set `self.MouseForwardScale` 1.0)
    (elif (> _returnvalue (- 1.0 _viewportedgethreshold))
      (set `self.MouseForwardScale` -1.0)
      (else
        (set `self.MouseForwardScale` 0.0)))))

(fn `UserConstructionScript`)